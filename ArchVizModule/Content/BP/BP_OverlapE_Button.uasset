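; BP_OverlapE_Button is a proximity trigger that shows the WBP_EButton widget while a Character is inside its sphere.
; Each begin overlap creates a new widget, stores it in UIRef, adds it to the viewport, and switches player 0 to Game and UI input with a visible cursor.
; End overlap only hides the widget; the nodes restoring game-only input and hiding the cursor are disconnected.
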(event OnComponentBeginOverlap(Sphere)
  (params (OverlappedComponent :type Primitive%20Component%20Object%20Reference) (OtherActor :type Actor%20Object%20Reference) (OtherComp :type Primitive%20Component%20Object%20Reference) (OtherBodyIndex :type Integer) (bFromSweep :type Boolean) (SweepResult :type Hit%20Result%20Structure%20%28by%20ref%29))
  (bind _returnvalue (Game|GetPlayerController 0))
  (Utilities|Casting|CastToCharacter OtherActor)
  (bind _returnvalue_2 (UserInterface|CreateWidget "/ArchVizModule/UI/Widgets/WBP_EButton.WBP_EButton_C"))
  (bind _output_get (Variables|Default|SetUIRef _returnvalue_2))
  (UserInterface|Viewport|AddtoViewport _output_get 0)
  (Widget|SetVisibility _returnvalue_2 "Visible")
  (Input|SetInputModeGameandUI _returnvalue 0 "DoNotLock" true false)
  (Variables|/Script/Engine.PlayerController|SetbShowMouseCursor _returnvalue true))

(event OnComponentEndOverlap(Sphere)
  (params (OverlappedComponent :type Primitive%20Component%20Object%20Reference) (OtherActor :type Actor%20Object%20Reference) (OtherComp :type Primitive%20Component%20Object%20Reference) (OtherBodyIndex :type Integer))
  (Utilities|Casting|CastToCharacter OtherActor)
  (Widget|SetVisibility (Variables|Default|GetUIRef) "Hidden"))

(event EventBeginPlay)

(event Collision|EventActorBeginOverlap
  (params (OtherActor :type Actor%20Object%20Reference)))

(event EventTick
  (params (DeltaSeconds :type Float%20%28single-precision%29)))

(fn ConstructionScript)