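; BP_OverlapAccesDeny is an access-denied indicator actor that reacts when a Character enters its trigger sphere.
; The static mesh starts hidden, becomes visible on Character overlap alongside a 2D CompileFailed sound, and hides again when the Character leaves.
; A DenialUI timeline with a ShakeZ track is present but never runs, so no shake occurs.
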(event OnComponentBeginOverlap(Sphere)
  (params (OverlappedComponent :type Primitive%20Component%20Object%20Reference) (OtherActor :type Actor%20Object%20Reference) (OtherComp :type Primitive%20Component%20Object%20Reference) (OtherBodyIndex :type Integer) (bFromSweep :type Boolean) (SweepResult :type Hit%20Result%20Structure%20%28by%20ref%29))
  (Utilities|Casting|CastToCharacter OtherActor)
  (Rendering|SetVisibility (Variables|Default|GetStaticMesh) true false)
  (Audio|PlaySound2D "/ArchVizModule/Sound/CompileFailed.CompileFailed" 1.0 1.0 0.0 0 0))

(event OnComponentEndOverlap(Sphere)
  (params (OverlappedComponent :type Primitive%20Component%20Object%20Reference) (OtherActor :type Actor%20Object%20Reference) (OtherComp :type Primitive%20Component%20Object%20Reference) (OtherBodyIndex :type Integer))
  (Utilities|Casting|CastToCharacter OtherActor)
  (Rendering|SetVisibility (Variables|Default|GetStaticMesh) false false))

(event EventBeginPlay
  (Rendering|SetVisibility (Variables|Default|GetStaticMesh) false false))

(fn ConstructionScript)