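; BP_OverlapScanner is a proximity trigger that shows a scanner UI while a Character is inside its Sphere.
; Each begin overlap by any Character creates a new WBP_Scanner widget, stores it in RefUI and adds it to the viewport.
; End overlap hides the stored widget without removing it.
; Disconnected DenialUI and failure-sound nodes never run.
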(event OnComponentBeginOverlap(Sphere)
  (params (OverlappedComponent :type Primitive%20Component%20Object%20Reference) (OtherActor :type Actor%20Object%20Reference) (OtherComp :type Primitive%20Component%20Object%20Reference) (OtherBodyIndex :type Integer) (bFromSweep :type Boolean) (SweepResult :type Hit%20Result%20Structure%20%28by%20ref%29))
  (Utilities|Casting|CastToCharacter OtherActor)
  (bind _returnvalue (UserInterface|CreateWidget "/ArchVizModule/UI/Widgets/WBP_Scanner.WBP_Scanner_C"))
  (Variables|Default|SetRefUI _returnvalue)
  (UserInterface|Viewport|AddtoViewport _returnvalue 0)
  (Widget|SetVisibility _returnvalue "Visible"))

(event OnComponentEndOverlap(Sphere)
  (params (OverlappedComponent :type Primitive%20Component%20Object%20Reference) (OtherActor :type Actor%20Object%20Reference) (OtherComp :type Primitive%20Component%20Object%20Reference) (OtherBodyIndex :type Integer))
  (Utilities|Casting|CastToCharacter OtherActor)
  (Widget|SetVisibility (Variables|Default|GetRefUI) "Hidden"))

(event EventBeginPlay)

(fn ConstructionScript)