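; BP_OverlapMenuScifi is a trigger actor that shows a sci-fi info menu while the third-person character stands inside its Sphere.
; On overlap it switches the character to the first-person camera, creates WBP_Scifi_Info and enables the cursor with Game and UI input.
; On exit it restores third-person view and game-only input, hides the widget and stops its audio.
; Each entry creates a new widget rather than reusing the hidden one.
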(event OnComponentBeginOverlap(Sphere)
  (params (OverlappedComponent :type Primitive%20Component%20Object%20Reference) (OtherActor :type Actor%20Object%20Reference) (OtherComp :type Primitive%20Component%20Object%20Reference) (OtherBodyIndex :type Integer) (bFromSweep :type Boolean) (SweepResult :type Hit%20Result%20Structure%20%28by%20ref%29))
  (bind _returnvalue (Game|GetPlayerController 0))
  (bind _asbp_third_person_character (Utilities|Casting|CastToBP_ThirdPersonCharacter OtherActor))
  (Default|CameraFPS _asbp_third_person_character)
  (bind _returnvalue_2 (UserInterface|CreateWidget "/ArchVizModule/Scifi_UI/WBP_Scifi_Info.WBP_Scifi_Info_C"))
  (bind _output_get (Variables|Default|SetRefUI1 _returnvalue_2))
  (UserInterface|Viewport|AddtoViewport _output_get 0)
  (Widget|SetVisibility _returnvalue_2 "Visible")
  (Input|SetInputModeGameandUI _returnvalue 0 "DoNotLock" true false)
  (Variables|/Script/Engine.PlayerController|SetbShowMouseCursor _returnvalue true))

(event OnComponentEndOverlap(Sphere)
  (params (OverlappedComponent :type Primitive%20Component%20Object%20Reference) (OtherActor :type Actor%20Object%20Reference) (OtherComp :type Primitive%20Component%20Object%20Reference) (OtherBodyIndex :type Integer))
  (bind _returnvalue (Game|GetPlayerController 0))
  (bind _refui1 (Variables|Default|GetRefUI1))
  (bind _allcompaudio (Variables|/ArchVizModule/Scifi_UI/WBP_Scifi_Info.WBP_Scifi_Info_C|GetAllCompAudio _refui1))
  (bind _asbp_third_person_character (Utilities|Casting|CastToBP_ThirdPersonCharacter OtherActor))
  (Default|CameraTPS _asbp_third_person_character)
  (Widget|SetVisibility _refui1 "Hidden")
  (Input|SetInputModeGameOnly _returnvalue false)
  (Variables|/Script/Engine.PlayerController|SetbShowMouseCursor _returnvalue false)
  (Utilities|IsValid _allcompaudio
    (:Is%20Valid
      (Class|ArchVizFunctionLibrary|StopAllAudio _allcompaudio))))

(event EventBeginPlay)

(event Collision|EventActorBeginOverlap
  (params (OtherActor :type Actor%20Object%20Reference)))

(event EventTick
  (params (DeltaSeconds :type Float%20%28single-precision%29)))

(fn ConstructionScript)