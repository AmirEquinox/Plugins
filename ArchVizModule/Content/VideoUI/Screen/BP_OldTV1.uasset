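; BP_OldTV1 is an old TV screen that plays a test video through a media player.
; Entering its sphere trigger opens the video on loop, and leaving closes the player.
; An Interact event uses a FlipFlop to alternate between playing the same video once and closing it, independently of the overlap state.
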(event OnComponentBeginOverlap(Sphere)
  (params (OverlappedComponent :type Primitive%20Component%20Object%20Reference) (OtherActor :type Actor%20Object%20Reference) (OtherComp :type Primitive%20Component%20Object%20Reference) (OtherBodyIndex :type Integer) (bFromSweep :type Boolean) (SweepResult :type Hit%20Result%20Structure%20%28by%20ref%29))
  (Media|MediaPlayer|OpenSource (Variables|Default|GetScreenMediaPlayer) "/Game/Movie/TestMedia1.TestMedia1")
  (Components|Timeline|SetLooping (Variables|Default|GetScreenMediaPlayer) true))

(event OnComponentEndOverlap(Sphere)
  (params (OverlappedComponent :type Primitive%20Component%20Object%20Reference) (OtherActor :type Actor%20Object%20Reference) (OtherComp :type Primitive%20Component%20Object%20Reference) (OtherBodyIndex :type Integer))
  (Media|MediaPlayer|Close (Variables|Default|GetScreenMediaPlayer) :!class /Script/MediaAssets.MediaPlayer))

(event EventBeginPlay)

(event EventInteract
  (bind _screenmediaplayer (Variables|Default|GetScreenMediaPlayer))
  (Utilities|FlowControl|FlipFlop
    (:A
      (Media|MediaPlayer|OpenSource _screenmediaplayer "/Game/Movie/TestMedia1.TestMedia1")
      ;[1 1 1] Don't Loop
      (Components|Timeline|SetLooping (Variables|Default|GetScreenMediaPlayer) false))
    (:B
      (Media|MediaPlayer|Close _screenmediaplayer :!class /Script/MediaAssets.MediaPlayer))))

(fn ConstructionScript)