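; BP_TVChannels is an in-game TV Blueprint that controls looping video playback on a screen Media Player.
; Interact uses a FlipFlop to alternate between opening the second playlist entry and closing the player.
; ChangeForward cycles the first two playlist entries through a looping MultiGate, while ChangeBackward is an empty stub.
; An older interact event toggles a single media source, and disconnected FlipFlop and MultiGate nodes remain unused.
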(event Custom|INterface%20Interact%20function
  (bind _screenmediaplayer (Variables|Default|GetScreenMediaPlayer))
  ;[1 1 1] Open Close TV old logic
  ;;[1 1 1] INteract Interace function
  (Utilities|FlowControl|FlipFlop
    (:A
      (Media|MediaPlayer|OpenSource _screenmediaplayer "/Game/Movie/videoplayback.videoplayback")
      (Components|Timeline|SetLooping (Variables|Default|GetScreenMediaPlayer) true))
    (:B
      (Media|MediaPlayer|Close _screenmediaplayer :!class /Script/MediaAssets.MediaPlayer))))

(event EventBeginPlay)

(event EventChangeBackward
  ;[1 1 1] Revese Playlist
)

(event EventChangeForward
  ;[1 1 1] Forward Playlist
  (Utilities|FlowControl|MultiGate false true 0 :!label _label
    (:Out%200
      (Class|MediaPlayer|OpenPlaylistIndex (Variables|Default|GetScreenMediaPlayer) "/Game/Movie/MediaPlaylist.MediaPlaylist")
      (Components|Timeline|SetLooping (Variables|Default|GetScreenMediaPlayer) true))
    (:Out%201
      (Class|MediaPlayer|OpenPlaylistIndex (Variables|Default|GetScreenMediaPlayer) "/Game/Movie/MediaPlaylist.MediaPlaylist" 1)
      (Components|Timeline|SetLooping (Variables|Default|GetScreenMediaPlayer) true)
      (goto _label Reset))))

(event EventInteract
  ;[1 1 1] Not interface check
  (Utilities|FlowControl|FlipFlop
    (:A
      (Class|MediaPlayer|OpenPlaylistIndex (Variables|Default|GetScreenMediaPlayer) "/Game/Movie/MediaPlaylist.MediaPlaylist" 1)
      (Components|Timeline|SetLooping (Variables|Default|GetScreenMediaPlayer) true))
    (:B
      (Media|MediaPlayer|Close (Variables|Default|GetScreenMediaPlayer) :!class /Script/MediaAssets.MediaPlayer))))

(fn ConstructionScript)