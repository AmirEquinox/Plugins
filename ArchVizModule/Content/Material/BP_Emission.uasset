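; Actor Blueprint that fades an emission material parameter on its Cube mesh in when a Character enters its Sphere trigger.
; BeginPlay creates a dynamic instance of the Cube's first material and applies it.
; The Emission timeline drives a variable-named scalar parameter between 0 and 1.
; It plays forward on Character overlap and reverses when any overlap ends, without a Character check.
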(event OnComponentBeginOverlap(Sphere)
  (params (OverlappedComponent :type Primitive%20Component%20Object%20Reference) (OtherActor :type Actor%20Object%20Reference) (OtherComp :type Primitive%20Component%20Object%20Reference) (OtherBodyIndex :type Integer) (bFromSweep :type Boolean) (SweepResult :type Hit%20Result%20Structure%20%28by%20ref%29))
  (Utilities|Casting|CastToCharacter OtherActor)
  (bind _emission (Timeline|Emission Play)
    (:Update
      (Rendering|Material|SetScalarParameterValue (Variables|Default|GetDynMatEmision) (Variables|Default|GetParameter%20Name) (Math|Float|Lerp 0.0 1.0 _emission) :!class /Script/Engine.MaterialInstanceDynamic))))

(event OnComponentEndOverlap(Sphere)
  (params (OverlappedComponent :type Primitive%20Component%20Object%20Reference) (OtherActor :type Actor%20Object%20Reference) (OtherComp :type Primitive%20Component%20Object%20Reference) (OtherBodyIndex :type Integer))
  (bind _emission (Timeline|Emission Reverse)
    (:Update
      (Rendering|Material|SetScalarParameterValue (Variables|Default|GetDynMatEmision) (Variables|Default|GetParameter%20Name) (Math|Float|Lerp 0.0 1.0 _emission) :!class /Script/Engine.MaterialInstanceDynamic))))

(event EventBeginPlay
  (bind _returnvalue (Rendering|Material|CreateDynamicMaterialInstance (Rendering|Material|GetMaterial (Variables|Default|GetCube) 0) "None" "None" :!class /Script/Engine.KismetMaterialLibrary))
  (bind _output_get (Variables|Default|SetDynMatEmision _returnvalue))
  (Rendering|Material|SetMaterial (Variables|Default|GetCube) 0 _output_get))

(event Collision|EventActorBeginOverlap
  (params (OtherActor :type Actor%20Object%20Reference)))

(event EventTick
  (params (DeltaSeconds :type Float%20%28single-precision%29)))

(fn ConstructionScript)